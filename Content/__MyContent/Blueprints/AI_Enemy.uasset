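; AI_Enemy is an enemy that follows pawns it sees and hurts the player on contact.
; PawnSensing triggers a simple move toward the seen pawn.
; A box overlap with the tagged FirstPersonCharacter applies instant damage capped at MaxDamage.
; While overlap lasts, Tick accumulates rate-based damage up to that cap, but multiplies the health change by zero, so only the initial hit lands.
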(event `self.PawnSensing.OnSeePawn`
  (params (Pawn :type "Pawn Object Reference"))
  ;[1 1 1] Enemy Follow
  (`AIBlueprintHelperLibrary.SimpleMoveToActor` (`self.GetController`) Pawn))

(event `self.ReceiveTick`
  (params (DeltaSeconds :type "Float (single-precision)"))
  (if (`self.Inside Volume`)
    (`self.Continue Damage`)))

(event `self.Box.OnComponentBeginOverlap`
  (params (OverlappedComponent :type "PrimitiveComponent Object Reference") (OtherActor :type "Actor Object Reference") (OtherComp :type "PrimitiveComponent Object Reference") (OtherBodyIndex :type Integer) (bFromSweep :type Boolean) (SweepResult :type "HitResult Structure (by ref)"))
  (if (`self.ActorHasTag` OtherActor "My Player")
    (bind _asfirst_person_character (cast `/Game/FirstPersonBP/Blueprints/FirstPersonCharacter` OtherActor))
    (set `self.Inside Volume` true)
    (set `self.My Player` _asfirst_person_character)
    (`self.Start Damage`)))

(event `self.Box.OnComponentEndOverlap`
  (params (OverlappedComponent :type "PrimitiveComponent Object Reference") (OtherActor :type "Actor Object Reference") (OtherComp :type "PrimitiveComponent Object Reference") (OtherBodyIndex :type Integer))
  (if (`self.ActorHasTag` OtherActor "My Player")
    (cast `/Game/FirstPersonBP/Blueprints/FirstPersonCharacter` OtherActor)
    (set `self.Inside Volume` false)))

(fn `Continue Damage`
  (bind _returnvalue (* (`self.Damage Rate`) (`GameplayStatics.GetWorldDeltaSeconds`)))
  (if (< (`self.Accum Damage`) (`self.Max Damage`))
    (set `self.Accum Damage` (+ _returnvalue (`self.Accum Damage`)))
    (`/Game/FirstPersonBP/Blueprints/FirstPersonCharacter.Change Health` (`self.My Player`) (* _returnvalue 0.0))))

(fn `Start Damage`
  (bind _output_get (set `self.Accum Damage` (`self.Instant Damage`)))
  (if (> _output_get (`self.Max Damage`))
    (set `self.Accum Damage` (`self.Max Damage`)))
  (`/Game/FirstPersonBP/Blueprints/FirstPersonCharacter.Change Health` (`self.My Player`) (* (`self.Accum Damage`) -1.0)))

(fn `UserConstructionScript`)