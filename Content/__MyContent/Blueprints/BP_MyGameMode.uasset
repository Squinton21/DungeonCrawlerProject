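; Game mode Blueprint that creates the game's main UI widgets and stores them on the BP_MyGameManager actor.
; On BeginPlay it caches the first BP_MyGameManager found in the level.
; A CreateUI function builds the Abandon, Success, Lose and HUD widgets, assigns each to a manager variable and adds all four to the viewport.
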(event `self.ReceiveBeginPlay`
  (bind _outactors (`GameplayStatics.GetAllActorsOfClass` "/Game/__MyContent/Blueprints/BP_MyGameManager.BP_MyGameManager_C"))
  (set `self.My Game Manager` (`|GetArrayItem` _outactors)))

(fn `Create UI`
  (bind _my_game_manager (`/Game/__MyContent/Blueprints/BP_MyFunctionLibrary.Get My Game Manager`))
  (bind _returnvalue (`|CreateWidget` "/Game/__MyContent/UI/Widget_Abandon.Widget_Abandon_C"))
  (bind _output_get (set `/Game/__MyContent/Blueprints/BP_MyGameManager.Widget Abandon` _returnvalue _my_game_manager))
  (`UserWidget.AddToViewport` _output_get 0)
  (bind _returnvalue_2 (`|CreateWidget` "/Game/__MyContent/UI/Widget_Success.Widget_Success_C"))
  (bind _output_get_2 (set `/Game/__MyContent/Blueprints/BP_MyGameManager.Widget Success` _returnvalue_2 _my_game_manager))
  (`UserWidget.AddToViewport` _output_get_2 0)
  (bind _returnvalue_3 (`|CreateWidget` "/Game/__MyContent/UI/Widget_Lose.Widget_Lose_C"))
  (bind _output_get_3 (set `/Game/__MyContent/Blueprints/BP_MyGameManager.Widget Lose` _returnvalue_3 _my_game_manager))
  (`UserWidget.AddToViewport` _output_get_3 0)
  (bind _returnvalue_4 (`|CreateWidget` "/Game/__MyContent/UI/Widget_HUD.Widget_HUD_C"))
  (bind _output_get_4 (set `/Game/__MyContent/Blueprints/BP_MyGameManager.Widget HUD` _returnvalue_4 _my_game_manager))
  (`UserWidget.AddToViewport` _output_get_4 0))

(fn `UserConstructionScript`)